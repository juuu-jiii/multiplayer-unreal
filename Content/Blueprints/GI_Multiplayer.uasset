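; Game Instance Blueprint that hosts multiplayer sessions through Advanced Sessions.
; The CreateSession event packs session name, map name and game mode into string session properties as extra settings, alongside player count and LAN choice.
; On success it opens the named map as a listen server, while failure only prints a message.
; A LoadLevel helper also opens maps with the listen option, but its only call here is unwired.
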(event Custom|Create%20Session
  (params (MaxPlayers :type Integer) (bUseLAN :type Boolean) (SessionName :type String) (MapName :type String) (GameMode :type String))
  (|AdvancedSession (Utilities|Array|MakeArray (Class|AdvancedSessionsLibrary|MakeLiteralSessionPropertyString "SessionName" SessionName) (Class|AdvancedSessionsLibrary|MakeLiteralSessionPropertyString "MapName" MapName) (Class|AdvancedSessionsLibrary|MakeLiteralSessionPropertyString "GameMode" GameMode)) (Game|GetPlayerController 0) MaxPlayers MaxPlayers bUseLAN true false true true true false false false true false true
    (:OnSuccess
      (Development|PrintString "Created session successfully" true true "(R=0.113357,G=1.000000,B=0.000000,A=1.000000)")
      (Game|OpenLevel(byName) (Utilities|String|StringToName MapName) true "listen") ; Add "listen" to options to make the level start listening for connections.
    )
    (:OnFailure
      (Development|PrintString "Failed to create session" true true "(R=1.000000,G=0.000000,B=0.018245,A=1.000000)"))))

(fn LoadLevel
  (params (LevelName :type String))
  (Game|OpenLevel(byName) (Utilities|String|StringToName LevelName) true "listen"))