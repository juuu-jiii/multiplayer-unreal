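; Player controller for the Tag game mode that gates pawn movement around round start and displays the round UI.
; On BeginPlay it sets game-only input and freezes the pawn by disabling its input until Unfreeze is called.
; Enter calls GM_Tag's Countdown, which only succeeds where the game mode exists, on the server.
; ShowCountdown, a reliable owning-client event, and ShowInfo add the countdown and time-remaining widgets.
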(event Custom|Unfreeze
  ;[1 1 1] Enable input for the pawn this controller references.
  (Input|EnableInput (Pawn|GetControlledPawn) self))

(event Custom|ShowCountdown
  ;[1 1 1] Set to reliably run on owning clients, so that the server (and only the server) becomes responsible for executing this event on all clients.
  (bind _returnvalue (Game|ConstructObjectfromClass "/Game/GameModes/Tag/UI_Countdown.UI_Countdown_C"))
  (UserInterface|Viewport|AddtoViewport _returnvalue 0))

(event Custom|ShowInfo
  ;[1 1 1] Display the time remaining in the current round.
  (bind _returnvalue (UserInterface|CreateWidget "/Game/GameModes/Tag/UI_Info.UI_Info_C"))
  (UserInterface|Viewport|AddtoViewport _returnvalue 0))

(event Custom|Freeze
  ;[1 1 1] Disable input for the pawn this controller references.
  (Input|DisableInput (Pawn|GetControlledPawn) self))

(event EventBeginPlay
  ;[1 1 1] When a session is created/joined set input mode to game so the engine begins registering controller input as game-related.
  ; Then, prevent movement on session start until server starts the game by pressing ENTER.
  (Input|SetInputModeGameOnly self)
  (CallFunction|Freeze))

(event EventTick
  (params (DeltaSeconds :type Float%20%28single-precision%29)))

(event Input|KeyboardEvents|Enter
  (params (Key :type Key%20Structure :default "None"))
  ;[1 1 1] Begin countdown when ENTER is pressed.
  (:Pressed
    (bind _asgm_tag (Utilities|Casting|CastToGM_Tag (Game|GetGameMode)))
    (Default|Countdown _asgm_tag)))

(fn ConstructionScript)