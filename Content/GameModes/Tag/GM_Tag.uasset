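; GM_Tag is the game mode for a multiplayer Tag match, running it from player join to level change.
; Each joining PC_Tag is stored and given a character at the PlayerStart tagged with its join index.
; A once-only countdown unfreezes all players, then a looping one-second timer decrements GS_Tag's CurrentTime to share with clients.
; At zero it freezes players, hides timers and server-travels to the next map.
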(event Custom|Countdown
  ;[1 1 1] Countdown -- executed when server presses ENTER (see PC_Tag)
  ;;[1 1 1] Prevent multiple overlapping countdowns from being started.
  ;; Alternatively: use a "Do Once" node.
  (if (not (Variables|Default|GetStarted))
    (for _array_element (Variables|Default|GetPlayers)
      (Default|ShowCountdown _array_element))
    ;;[1 1 1] Unfreeze all players after 3 seconds i.e., once the countdown timer is finished
    (Variables|Default|SetStarted true)
    (Utilities|FlowControl|Delay 3.0)
    (CallFunction|Unfreeze)))

(event Custom|Unfreeze
  ;[1 1 1] Game start logic
  ;;[1 1 1] Loop through all player controllers and enable control input.
  (for _array_element (Variables|Default|GetPlayers)
    (Default|Unfreeze _array_element))
  ;;[1 1 1] Initialise GS_Tag.CurrentTime to be equal to MatchTime .
  (Variables|/Game/GameModes/Tag/GS_Tag.GS_Tag_C|SetCurrentTime (Variables|Default|GetGS%20Tag) (Variables|Default|GetMatchTime))
  ;[1 1 1] Game update logic
  ;;[1 1 1] Count is fired every second, decrementing current time by 1.
  (bind _returnvalue (Utilities|Time|SetTimerbyEvent (delegate Custom|Count) 1.0 true))
  (CallFunction|ShowTimers))

(event Custom|Count
  ;[1 1 1] Game update logic
  ;;[1 1 1] Count is fired every second, decrementing current time by 1.
  (bind _result (Math|Integer|DecrementInt (Variables|/Game/GameModes/Tag/GS_Tag.GS_Tag_C|GetCurrentTime (Variables|Default|GetGS%20Tag)))
    (:%20%20
      ;;[1 1 1] When timer hits zero, pause it so it doesn't go into the negatives. Then, disable player input across all controllers.
      (if (== _result 0)
        (Utilities|Time|PauseTimerbyHandle (stale Custom|Unfreeze _returnvalue))
        (CallFunction|Freeze)
        (CallFunction|HideTimers)
        (Utilities|FlowControl|Delay 2.0)
        (CallFunction|Travelto "ThirdPersonMap_Duplicate_2")))))

(event Custom|ShowTimers
  ;[1 1 1] Loop through all player controllers and display their timer widgets.
  (for _array_element (Variables|Default|GetPlayers)
    (Default|ShowInfo _array_element)))

(event Custom|Freeze
  ;[1 1 1] Loop through all player controllers and disable control input.
  (for _array_element (Variables|Default|GetPlayers)
    (Default|Freeze _array_element)))

(event Custom|TravelTo
  (params (Level%20Name :type String))
  (Development|ExecuteConsoleCommand (Utilities|String|Append "servertravel " Level%20Name) 0))

(event Custom|HideTimers
  ;[1 1 1] Loop through all player controllers and hide their timer widgets.
  (for _array_element (Variables|Default|GetPlayers)
    (Default|HideInfo _array_element)))

(event Custom|InitGSTag
  ;[1 1 1] Get a reference to the tag GameState blueprint.
  ; GameStates are useful to share server values with all clients.
  ; (The Game State Class in this blueprint was set to point at GS_Tag)
  (if (not (Utilities|IsValid (Variables|Default|GetGS%20Tag)))
    (bind _asgs_tag (Utilities|Casting|CastToGS_Tag (Game|GetGameState)))
    (Variables|Default|SetGS%20Tag _asgs_tag)))

(event EventBeginPlay)

(event EventTick
  (params (DeltaSeconds :type Float%20%28single-precision%29)))

(event EventPostLogin
  (params (NewPlayer :type Player%20Controller%20Object%20Reference))
  ;[1 1 1] Handle a new player joining the game.
  ;;[1 1 1] Both of these events handle players joining a session. They contain a reference to the joining player controller.
)

(event EventHandleStartingNewPlayer
  (params (NewPlayer :type Player%20Controller%20Object%20Reference))
  ;[1 1 1] Handle a new player joining the game.
  ;;[1 1 1] Both of these events handle players joining a session. They contain a reference to the joining player controller.
  (CallFunction|InitGSTag)
  (bind _aspc_tag (Utilities|Casting|CastToPC_Tag NewPlayer))
  (Utilities|Array|Add (Variables|Default|GetPlayers) _aspc_tag)
  ;;[1 1 1] Spawn a ThirdPersonCharacter Actor at the location of the assigned PlayerStart.
  (bind _returnvalue (Game|SpawnActorfromClass "/Game/ThirdPerson/Blueprints/BP_ThirdPersonCharacter.BP_ThirdPersonCharacter_C" (Transformation|GetActorTransform (Class|GameModeBase|FindPlayerStart NewPlayer (Utilities|String|ToString(Integer) (- (Utilities|Array|Length (Variables|Default|GetPlayers)) 1)))) "Undefined" 0 0))
  (Pawn|Possess NewPlayer _returnvalue) ; Set the joining player controller\nto possess the newly-spawned\nThirdPersonCharacter Actor.
)

(fn ConstructionScript)